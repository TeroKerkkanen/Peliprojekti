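; GainFullLifeEffect is an effect Blueprint that restores the player character's LifeForce when ApplyEffect is called.
; It plays a laser-shot sound at the world origin and disables player 0's input for a one-second delay.
; If LifeForce is below 1.0, it then adds FullLife scaled by elapsed game time, caps the result at 1.0 and sets its own Speed variable to a fixed value.
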(event `self.ApplyEffect`
  (params (PlayerCharacter :type "/Game/Blueprints/BB_MyCharacter Object Reference"))
  (bind _returnvalue (`GameplayStatics.GetPlayerController` 0))
  (bind _returnvalue_2 (`GameplayStatics.GetPlayerCharacter` 0))
  (bind _lifeforce (`/Game/Blueprints/BB_MyCharacter.lifeForce` PlayerCharacter))
  (bind _returnvalue_3 (+ _lifeforce (* (/ (`KismetSystemLibrary.GetGameTimeInSeconds`) 5.0) (`self.FullLife`))))
  (`GameplayStatics.PlaySoundAtLocation` "/Game/Sounds/space_laser_shot.space_laser_shot")
  (`self.DisableInput` _returnvalue_2 _returnvalue)
  (`KismetSystemLibrary.Delay` 1.0)
  (`self.EnableInput` _returnvalue_2 _returnvalue)
  (if (< _lifeforce 1.0)
    ;[1 1 1] Check wheather sum of boost and life force is on maximum or not and actually update characters life force accordingly
    (if (<= _returnvalue_3 1.0)
      (set `/Game/Blueprints/BB_MyCharacter.lifeForce` _returnvalue_3 PlayerCharacter)
      (else
        (set `/Game/Blueprints/BB_MyCharacter.lifeForce` 1.0 PlayerCharacter)))
    (set `self.Speed` 500.0)))

(fn `UserConstructionScript`
  (`parent.UserConstructionScript`))