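; DrainLifeEffect is an effect actor whose ApplyEffect event is meant to drain the player character's LifeForce.
; The drain is Lifedrain scaled by total game time over five, so it grows as play goes on.
; LifeForce is written only when the result falls below zero, leaving the clamp to one unreachable.
; Every reachable path sets Speed to a fixed value, and no other event has active logic.
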(event `self.Apply effect`
  (params (`Player character` :type "/Game/Blueprints/BB_MyCharacter Object Reference"))
  (bind _returnvalue (- (`/Game/Blueprints/BB_MyCharacter.lifeForce` `Player character`) (* (/ (`KismetSystemLibrary.GetGameTimeInSeconds`) 5.0) (`self.lifedrain`))))
  ;[1 1 1] Check wheather players is not on  maximum before boost
  (if (< _returnvalue 0.0)
    ;[1 1 1] Check wheather sum of boost and life force is on maximum or not and actually update characters life force accordingly
    (if (<= _returnvalue 1.0)
      (set `/Game/Blueprints/BB_MyCharacter.lifeForce` _returnvalue `Player character`)
      (set `self.Speed` 50.0)
      (else
        (set `/Game/Blueprints/BB_MyCharacter.lifeForce` 1.0 `Player character`)))
    (else
      (set `self.Speed` 50.0))))

(fn `UserConstructionScript`
  (`parent.UserConstructionScript`))