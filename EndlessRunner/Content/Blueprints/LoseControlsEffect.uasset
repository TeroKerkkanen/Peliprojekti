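; LoseControlsEffect is an effect Blueprint that briefly takes away the player's controls.
; Its ApplyEffect event plays a laser shot sound at the world origin, then disables input on player character 0.
; After a one-second delay it re-enables that input.
; The BeginPlay, overlap and Tick events are disabled stubs.
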(event `self.Apply effect`
  (params (`Player character` :type "/Game/Blueprints/BB_MyCharacter Object Reference"))
  (bind _returnvalue (`GameplayStatics.GetPlayerController` 0))
  (bind _returnvalue_2 (`GameplayStatics.GetPlayerCharacter` 0))
  (`GameplayStatics.PlaySoundAtLocation` "/Game/Sounds/space_laser_shot.space_laser_shot")
  (`self.DisableInput` _returnvalue_2 _returnvalue)
  (`KismetSystemLibrary.Delay` 1.0)
  (`self.EnableInput` _returnvalue_2 _returnvalue))

(fn `UserConstructionScript`
  (`parent.UserConstructionScript`))