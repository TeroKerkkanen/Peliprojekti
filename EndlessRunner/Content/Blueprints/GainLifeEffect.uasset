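; GainLifeEffect is an effect Blueprint that restores a player character's LifeForce.
; ApplyEffect acts only when LifeForce is below 1.0, adding a boost and capping the result at 1.0.
; The boost is the Effect value scaled by elapsed game time, so it grows the longer the game runs.
; After a boost is applied, it also sets Speed to a fixed value.
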(event `self.ApplyEffect`
  (params (PlayerCharacter :type "/Game/Blueprints/BB_MyCharacter Object Reference"))
  (bind _lifeforce (`/Game/Blueprints/BB_MyCharacter.lifeForce` PlayerCharacter))
  (bind _returnvalue (+ _lifeforce (* (/ (`KismetSystemLibrary.GetGameTimeInSeconds`) 5.0) (`self.Effect`))))
  ;[1 1 1] Check wheather players is not on  maximum before boost
  (if (< _lifeforce 1.0)
    ;[1 1 1] Check wheather sum of boost and life force is on maximum or not and actually update characters life force accordingly
    (if (<= _returnvalue 1.0)
      (set `/Game/Blueprints/BB_MyCharacter.lifeForce` _returnvalue PlayerCharacter)
      (else
        (set `/Game/Blueprints/BB_MyCharacter.lifeForce` 1.0 PlayerCharacter)))
    (set `self.Speed` 500.0)))

(fn `UserConstructionScript`
  (`parent.UserConstructionScript`))