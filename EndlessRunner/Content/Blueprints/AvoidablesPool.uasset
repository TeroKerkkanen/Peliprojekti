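; AvoidablesPool is an object pool of side-scrolling obstacles that move right to left across the screen.
; CreateAvoidable spawns a random Avoidable class at the start X and a random height until the cap is reached, with game time affecting its random speed range.
; UpdateAvoidables shifts each pooled obstacle left by its speed, recycling those past the left limit with a new height and speed.
; Its own events are empty.
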(fn `CreateAvoidable`
  (bind _avoidables (`self.Avoidables`))
  ;[1 1 1] Only create avoidables if max amount not been reached
  (if (< (`self.numberofAvoidables`) (`self.maxNumberofAvoidables`))
    ;[1 1 1] Create avoidable in the scene and adjust its position and speed
    (bind _returnvalue (`|SpawnActorFromClass` (`|GetArrayItem` _avoidables (`KismetMathLibrary.RandomIntegerInRange` 0 (`KismetArrayLibrary.Array_LastIndex` _avoidables))) (`KismetMathLibrary.MakeTransform` (`KismetMathLibrary.MakeVector` (`self.AvoidableStartX`) 0.0 (`KismetMathLibrary.RandomFloatInRange` 150.0 900.0))) "Undefined" "OverrideRootScale" null null))
    (bind _asavoidable (cast `/Game/Blueprints/Avoidable` _returnvalue))
    (bind _speed (`/Game/Blueprints/Avoidable.Speed` _asavoidable))
    (set `/Game/Blueprints/Avoidable.Speed` (`KismetMathLibrary.RandomFloatInRange` (/ _speed (/ (`KismetSystemLibrary.GetGameTimeInSeconds`) 10.0)) _speed) _asavoidable)
    ;[1 1 1] Add created avoidable to the pool and increment counter
    (`KismetArrayLibrary.Array_Insert` (`self.thePool`) _asavoidable (`self.numberofAvoidables`))
    (`/Engine/EditorBlueprintResources/StandardMacros.IncrementInt` (`self.numberofAvoidables`))))

(fn `UpdateAvoidables`
  (locals (arrayElement :type "PaperSpriteActor Object Reference") (arrayIndex :type Integer))
  ;[1 1 1] Update each avoidable in the pool
  (for _array_element (`self.thePool`)
    ;[1 1 1] Check whether avoidable has travelled far enough to the left of the screen in order to be valid for reappering again from the right side of the screen
    (set `local.arrayElement` _array_element)
    (bind _rootcomponent (`Actor.RootComponent` _array_element))
    (if (< (.x (`SceneComponent.K2_GetComponentLocation` _rootcomponent)) (- 0.0 (`self.AvoidableStartX`)))
      ;[1 1 1] Create avoidable into the scene and adjust it's position and speed
      (`SceneComponent.K2_SetWorldLocation` (`Actor.RootComponent` (`local.arrayElement`)) (`KismetMathLibrary.MakeVector` (`self.AvoidableStartX`) 0.0 (`KismetMathLibrary.RandomFloatInRange` 150.0 900.0)) false false)
      (bind _asavoidable (cast `/Game/Blueprints/Avoidable` (`local.arrayElement`)))
      (set `/Game/Blueprints/Avoidable.Speed` (`KismetMathLibrary.RandomFloatInRange` 5.0 25.0) _asavoidable)
      (else
        ;[1 1 1] If not too far on the left just move the avoidable
        (bind _asavoidable_2 (cast `/Game/Blueprints/Avoidable` _array_element))
        (`SceneComponent.K2_AddWorldOffset` _rootcomponent (`KismetMathLibrary.MakeVector` (- 0.0 (`/Game/Blueprints/Avoidable.Speed` _asavoidable_2))) false false)))))

(fn `UserConstructionScript`)